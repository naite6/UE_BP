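; Player character Blueprint with camera-relative movement, look, jump, run, and a sword that can be drawn, sheathed and swung in combos.
; BeginPlay spawns the sword on a holster socket; equip and sheath events set state flags, move it between hand and holster sockets, and restore movement.
; Attacks play montages from an array, with Lock/UnLock opening an input window that queues the next hit for NextCombo.
; Movement and jumping are blocked while attacking, drawing or sheathing.
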(event Custom|NextCombo
  (bind _combo_index (Variables|Default|GetCombo_Index))
  (if (Variables|Default|GetCombo_Next)
    (Variables|Default|SetCombo_Next false)
    (Math|Integer|IncrementInt _combo_index
      (:%20%20
        (Animation|PlayAnimMontage (Utilities|Array|Get(acopy) (Variables|Default|GetCombo_Montages) _combo_index) 1.0 "None")))))

(event Custom|Lock
  (Variables|Default|SetCombo_Enable false))

(event Custom|UnLock
  (Variables|Default|SetCombo_Enable true))

(event Custom|EndAttack
  (Variables|Default|SetCanAttack true)
  (Variables|Default|SetCanMove true)
  (Variables|Default|SetCombo_Index 0))

(event Input|ActionEvents|InputActionAttack
  (params (Key :type Key%20Structure :default "None"))
  (:Pressed
    (if (Variables|Default|GetCombo_Enable)
      (Variables|Default|SetCombo_Enable false)
      (Variables|Default|SetCombo_Next true)
      (elif (and (Variables|Default|GetDrawn) (Variables|Default|GetCanAttack))
        (Variables|Default|SetCanAttack false)
        (Variables|Default|SetCanMove false)
        (Animation|PlayAnimMontage (Utilities|Array|Get(acopy) (Variables|Default|GetCombo_Montages)) 1.0 "None")))))

(fn ConstructionScript)

(event EventBeginPlay
  (bind _returnvalue (Game|SpawnActorfromClass "/Game/Blueprints/WeaPon/BP_Sword.BP_Sword_C" (Math|Transform|MakeTransform "0, 0, 0") "Undefined" self 0))
  (bind _output_get (Variables|Default|SetSword _returnvalue))
  (Transformation|AttachComponentToComponent _output_get (Variables|Character|GetMesh) "Holster_Sword" "KeepRelative" "KeepRelative" "KeepRelative" true))

(event Input|ActionEvents|InputActionJump
  (params (Key :type Key%20Structure :default "None"))
  ;[1 1 1] 점프
  (:Pressed
    (if (Variables|Default|GetCanMove)
      (Character|Jump))))

(event Input|ActionEvents|InputActionRun
  (params (Key :type Key%20Structure :default "None"))
  (bind _charactermovement (Variables|Character|GetCharacterMovement))
  ;[1 1 1] 달리기
  (:Pressed
    (Variables|/Script/Engine.CharacterMovementComponent|SetMaxWalkSpeed _charactermovement 1e+03))
  (:Released
    (Variables|/Script/Engine.CharacterMovementComponent|SetMaxWalkSpeed _charactermovement 6e+02)))

(event Input|AxisEvents|InputAxisMoveFoward
  (params (AxisValue :type Float%20%28single-precision%29))
  ;[1 1 1] 움직임
  (if (Variables|Default|GetCanMove)
    (Pawn|Input|AddMovementInput (Math|Vector|GetForwardVector (Math|Rotator|MakeRotator 0.0 0.0 (.yaw (Pawn|GetControlRotation :!class /Script/Engine.Pawn)))) AxisValue false)))

(event Input|AxisEvents|InputAxisMoveLeftRight
  (params (AxisValue :type Float%20%28single-precision%29))
  ;[1 1 1] 움직임
  (if (Variables|Default|GetCanMove)
    (Pawn|Input|AddMovementInput (Math|Vector|GetRightVector (Math|Rotator|MakeRotator 0.0 0.0 (.yaw (Pawn|GetControlRotation :!class /Script/Engine.Pawn)))) AxisValue false)))

(event Input|AxisEvents|InputAxisVerticallLook
  (params (AxisValue :type Float%20%28single-precision%29))
  ;[1 1 1] 시점
  (Pawn|Input|AddControllerPitchInput AxisValue))

(event Input|AxisEvents|InputAxisHorizontalLook
  (params (AxisValue :type Float%20%28single-precision%29))
  ;[1 1 1] 시점
  (Pawn|Input|AddControllerYawInput AxisValue))

(event Custom|Equip
  ;[1 1 1] Equip
  (Variables|Default|SetDrawing true)
  (Variables|Default|SetCanMove false))

(event Custom|BeginEquid
  ;[1 1 1] Equip
  (Transformation|AttachComponentToComponent (Variables|Default|GetSword) (Variables|Character|GetMesh) "Hand_Sword" "KeepRelative" "KeepRelative" "KeepRelative" true))

(event Custom|EndEquid
  ;[1 1 1] Equip
  (Variables|Default|SetDrawing false)
  (Variables|Default|SetDrawn true)
  (Variables|Default|SetCanMove true))

(event Custom|EndSheath
  ;[1 1 1] Sheath
  (Variables|Default|SetSheathing false)
  (Variables|Default|SetDrawn false)
  (Variables|Default|SetCanMove true))

(event Custom|Sheath
  ;[1 1 1] Sheath
  (Variables|Default|SetSheathing true)
  (Variables|Default|SetCanMove false))

(event Custom|BeginSheath
  ;[1 1 1] Sheath
  (Transformation|AttachComponentToComponent (Variables|Default|GetSword) (Variables|Character|GetMesh) "Holster_Sword" "KeepRelative" "KeepRelative" "KeepRelative" true))

(event Input|ActionEvents|InputActionSword
  (params (Key :type Key%20Structure :default "None"))
  ;[1 1 1] Sword
  (:Pressed
    (if (Variables|Default|GetDrawn)
      (CallFunction|Sheath)
      (else
        (CallFunction|Equip)))))