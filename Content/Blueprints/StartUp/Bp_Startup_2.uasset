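; Bp_Startup_2 is a startup-folder actor that spins itself and a child mesh continuously.
; Each tick it adds yaw to StaticMesh2's relative rotation, turns the whole actor more slowly, and resets StaticMesh's relative rotation to zero.
; The increments are per frame, not scaled by delta time, so spin speed follows frame rate.
; An actor-movement node is left unconnected, and BeginPlay and the construction script are empty.
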(event EventBeginPlay)

(event EventTick
  (params (DeltaSeconds :type Float%20%28single-precision%29))
  (bind _staticmesh2 (Variables|Default|GetStaticMesh2))
  (Utilities|FlowControl|Sequence
    (:then_0
      (Transformation|SetRelativeRotation _staticmesh2 (Math|Rotator|MakeRotator 0.0 0.0 (+ (.yaw (Variables|/Script/Engine.SceneComponent|GetRelativeRotation _staticmesh2)) 5.0)) false false))
    (:then_1
      (Transformation|SetActorRotation (Math|Rotator|MakeRotator 0.0 0.0 (+ (.yaw (Transformation|GetActorRotation)) 1.0))))
    (:then_2
      (Transformation|SetRelativeRotation (Variables|Default|GetStaticMesh) "0, 0, 0" false false))))

(fn ConstructionScript)